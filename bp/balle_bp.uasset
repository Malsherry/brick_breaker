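; Ball actor for a brick-breaker game, launched along X with a velocity-change impulse on BeginPlay.
; Each hit raises its speed slightly and clamps physics velocity to exactly that magnitude, preserving direction.
; Hitting a "brique" with durability 1 updates the score on the paddle pawn (barre_bp).
; On destruction, it asks the spawner for a new ball if lives remain, otherwise shows the Game Over widget.
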(event `self.ReceiveBeginPlay`
  (`PrimitiveComponent.AddImpulse` (`self.balle`) (1000.0 0.0 0.0) "None" true)
  (bind _asbarre_bp (cast `/Game/bp/barre_bp` (`GameplayStatics.GetPlayerPawn` 0)))
  (set `self.As Barre Bp` _asbarre_bp))

(event `self.ReceiveHit`
  (params (MyComp :type "PrimitiveComponent Object Reference") (Other :type "Actor Object Reference") (OtherComp :type "PrimitiveComponent Object Reference") (bSelfMoved :type Boolean) (HitLocation :type "Vector Structure") (HitNormal :type "Vector Structure") (NormalImpulse :type "Vector Structure") (Hit :type "HitResult Structure (by ref)"))
  (bind _balle (`self.balle`))
  (bind _ballspeed (`self.ballspeed`))
  (set `self.ballspeed` (+ (`self.ballspeed`) 5.0))
  (bind _returnvalue (`PrimitiveComponent.GetPhysicsLinearVelocity` _balle "None"))
  (`PrimitiveComponent.SetPhysicsLinearVelocity` _balle (`KismetMathLibrary.ClampVectorSize` _returnvalue _ballspeed _ballspeed) false "None")
  (if (`self.ActorHasTag` Other "brique")
    (bind _asbrique_bp (cast `/Game/bp/brique_bp` Other))
    (if (== (`/Game/bp/brique_bp.durabilite_brique` _asbrique_bp) 1)
      (`/Game/bp/score_bp.UpdateScore` (`/Game/bp/barre_bp.score` (`self.As Barre Bp`))))))

(event `self.ReceiveDestroyed`
  (if (> (`/Game/bp/barre_bp.lives` (`self.As Barre Bp`)) 0)
    (`/Game/bp/spawn_bp.spawnball` (`self.ballspawnref`))
    (else
      (bind _returnvalue (`|CreateWidget` "/Game/bp/gameover_bp.gameover_bp_C"))
      (`UserWidget.AddToViewport` _returnvalue 0))))

(fn `UserConstructionScript`)
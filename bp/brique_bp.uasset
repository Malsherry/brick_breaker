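; Destructible brick Blueprint for a brick-breaker game, with a durability counter that drops each time a balle_bp ball hits it.
; UpdateCouleur maps durability to a green, yellow or red material, both at construction and after each non-lethal hit.
; At zero durability the brick spawns an explosion, destroys itself and plays a sound.
; It then searches for remaining Brique_bp actors and shows the Win_bp widget if none are left.
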(event `self.ReceiveHit`
  (params (MyComp :type "PrimitiveComponent Object Reference") (Other :type "Actor Object Reference") (OtherComp :type "PrimitiveComponent Object Reference") (bSelfMoved :type Boolean) (HitLocation :type "Vector Structure") (HitNormal :type "Vector Structure") (NormalImpulse :type "Vector Structure") (Hit :type "HitResult Structure (by ref)"))
  (cast `/Game/bp/balle_bp` Other)
  (bind _result (`/Engine/EditorBlueprintResources/StandardMacros.DecrementInt` (`self.durabilite_brique`))
    (:`  `
      (if (== _result 0)
        (`GameplayStatics.SpawnEmitterAtLocation` "/Game/StarterContent/Particles/P_Explosion.P_Explosion" (`self.K2_GetActorLocation`))
        (`self.K2_DestroyActor`)
        (`GameplayStatics.PlaySound2D` "/Game/sounds/Undertale_Audio_Files_210_-_snd-bombsplosion.Undertale_Audio_Files_210_-_snd-bombsplosion" 1.0 1.0 0.0 null null)
        (bind _outactors (`GameplayStatics.GetAllActorsOfClass` "brique_bp_C"))
        (if (== (`KismetArrayLibrary.Array_Length` _outactors) 0)
          (bind _returnvalue (`|CreateWidget` "/Game/bp/win_bp.win_bp_C"))
          (`UserWidget.AddToViewport` _returnvalue 0))
        (else
          (`GameplayStatics.PlaySound2D` "/Game/sounds/Undertale_Audio_Files_146_-_mus-sfx-a-grab.Undertale_Audio_Files_146_-_mus-sfx-a-grab" 1.0 1.0 0.0 null null)
          (`self.Update_couleur`))))))

(fn `Update_couleur`
  (bind _brique (`self.brique`))
  (switch `int` (`self.durabilite_brique`)
    (:`1`
      (`PrimitiveComponent.SetMaterial` _brique 0 "/Game/materials/vert.vert"))
    (:`2`
      (`PrimitiveComponent.SetMaterial` _brique 0 "/Game/materials/jaune.jaune"))
    (:`3`
      (`PrimitiveComponent.SetMaterial` _brique 0 "/Game/materials/rouge.rouge"))))

(fn `UserConstructionScript`
  (`self.Update_couleur`))
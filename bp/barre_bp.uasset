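; Player-controlled paddle pawn for a brick-breaker game (casse-brique).
; On BeginPlay it hides the cursor, switches to game-only input, adds the Enhanced Input mapping context and puts the score widget on screen.
; The move input action slides the Barre component along local Z with a swept offset scaled by VitesseBarre, so collisions block it.
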(event `self.ReceiveBeginPlay`
  (bind _returnvalue (`GameplayStatics.GetPlayerController` 0))
  (set `PlayerController.bShowMouseCursor` false _returnvalue)
  (`WidgetBlueprintLibrary.SetInputMode_GameOnly` _returnvalue)
  (bind _asplayer_controller (cast `PlayerController` (`self.GetController`)))
  (bind _returnvalue_2 (pcsubsystem `EnhancedInputLocalPlayerSubsystem` _asplayer_controller))
  (`/Engine/EditorBlueprintResources/StandardMacros.IsValid` _returnvalue_2
    (:`Is Valid`
      (`EnhancedInputSubsystemInterface.AddMappingContext` _returnvalue_2 "/Game/controls/controles_cassebrique.controles_cassebrique" 0 (struct))
      (bind _returnvalue_3 (`|GenericCreateObject` "/Game/bp/score_bp.score_bp_C"))
      (bind _output_get (set `self.score` _returnvalue_3))
      (`UserWidget.AddToViewport` _output_get 0))))

(event `EnhancedInput|/Game/controls/move_IA`
  (params (ActionValue :type "Float (double-precision)") (ElapsedSeconds :type "Float (double-precision)") (TriggeredSeconds :type "Float (double-precision)") (InputAction :type "InputAction Object Reference" :default "/Game/controls/move_IA.move_IA"))
  (:`Triggered`
    (`SceneComponent.K2_AddLocalOffset` (`self.barre`) (`KismetMathLibrary.MakeVector` 0.0 0.0 (* ActionValue (`self.vitesse_barre`))) true false)))

(fn `UserConstructionScript`)